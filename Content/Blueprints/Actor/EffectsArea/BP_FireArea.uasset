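; BP_FireArea is an area-effect actor that puts the GE_FireArea gameplay effect on actors inside its Box.
; On begin overlap, any actor with an Ability System Component applies a level 1 spec of the effect to itself.
; The returned handle is stored in one ActiveGameplayEffect variable, shared by all overlapping actors.
; On end overlap, that handle is used to remove all stacks from the leaving actor's component.
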(event OnComponentBeginOverlap(Box)
  (params (OverlappedComponent :type Primitive%20Component%20Object%20Reference) (OtherActor :type Actor%20Object%20Reference) (OtherComp :type Primitive%20Component%20Object%20Reference) (OtherBodyIndex :type Integer) (bFromSweep :type Boolean) (SweepResult :type Hit%20Result%20Structure%20%28by%20ref%29))
  (bind _returnvalue (Ability|GetAbilitySystemComponent OtherActor))
  (Utilities|IsValid _returnvalue
    (:Is%20Valid
      (bind _returnvalue_2 (GameplayEffects|ApplyGameplayEffectSpecToSelf _returnvalue (GameplayEffects|MakeOutgoingSpec _returnvalue "/Game/Blueprints/Actor/EffectsArea/GE_FireArea.GE_FireArea_C" 1.0 (GameplayEffects|MakeEffectContext _returnvalue))))
      (Variables|Default|SetActiveGameplayEffect _returnvalue_2))))

(event OnComponentEndOverlap(Box)
  (params (OverlappedComponent :type Primitive%20Component%20Object%20Reference) (OtherActor :type Actor%20Object%20Reference) (OtherComp :type Primitive%20Component%20Object%20Reference) (OtherBodyIndex :type Integer))
  (bind _returnvalue (Ability|GetAbilitySystemComponent OtherActor))
  (Utilities|IsValid _returnvalue
    (:Is%20Valid
      (GameplayEffects|RemoveActiveGameplayEffect _returnvalue (Variables|Default|GetActiveGameplayEffect) -1))))

(fn ConstructionScript)