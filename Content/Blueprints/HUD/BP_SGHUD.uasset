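; BP_SGHUD is a HUD Blueprint that toggles the container inventory screen.
; ToggleShowContainer first calls RemoveCharacterSheet, then either removes an existing container widget or creates WBP_ContainerInventory with the supplied inventory.
; Opening shows the cursor, switches input to game-and-UI and plays a sound; closing restores game-only input and hides the cursor.
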(event EventToggleShowContainer
  (params (ContainerInventory :type Inventory%20Component%20Object%20Reference))
  (bind _returnvalue (Game|GetPlayerController 0))
  (bind _returnvalue_2 (Game|GetPlayerController 0))
  (Class|SGHUD|RemoveCharacterSheet)
  (Utilities|IsValid (Variables|Default|GetContainerWidget)
    (:Is%20Valid
      (Widget|RemovefromParent (Variables|Default|GetContainerWidget))
      (Input|SetInputModeGameOnly _returnvalue false)
      (Variables|/Script/Engine.PlayerController|SetbShowMouseCursor _returnvalue false)
      (Variables|Default|SetContainerWidget 0)
      (Variables|Default|SetbIsContainerOpen false))
    (:Is%20Not%20Valid
      (bind _returnvalue_3 (UserInterface|CreateWidget "/Game/Blueprints/HUD/Inventory/WBP_ContainerInventory.WBP_ContainerInventory_C" 0 ContainerInventory))
      (bind _output_get (Variables|Default|SetContainerWidget _returnvalue_3))
      (UserInterface|Viewport|AddtoViewport _output_get 0)
      (Input|SetInputModeGameandUI _returnvalue_2 0 "DoNotLock" true false)
      (Variables|/Script/Engine.PlayerController|SetbShowMouseCursor _returnvalue_2 true)
      (Variables|Default|SetbIsContainerOpen true)
      (Audio|PlaySound2D "/Game/Assets/Sounds/Inventory/OpenInven.OpenInven" 1.0 1.0 0.0 0 0))))

(fn ConstructionScript)